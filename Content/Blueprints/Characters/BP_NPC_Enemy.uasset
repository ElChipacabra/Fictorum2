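; BP_NPC_Enemy is an enemy NPC character with an overhead attribute slider widget and a sword in its right hand.
; Construction registers the sword child actor as the right-hand item and takes ownership of it.
; BeginPlay binds the slider widget to this character and flags it as on an enemy.
; On death, it removes the widget, then detaches the sword and enables physics so it drops.
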(event EventBeginPlay
  (|CallParentFunction)
  (bind _asui_attribute_slider (Utilities|Casting|CastToUI_AttributeSlider (UserInterface|GetUserWidgetObject (Variables|Default|GetWidget))))
  (Variables|/Game/UI/UI_AttributeSlider.UI_AttributeSlider_C|SetCharacter _asui_attribute_slider self)
  (Variables|/Game/UI/UI_AttributeSlider.UI_AttributeSlider_C|SetOnEnemy _asui_attribute_slider true))

(event EventDeath
  (|CallParentFunction)
  (Widget|RemovefromParent (UserInterface|GetUserWidgetObject (Variables|Default|GetWidget)))
  (bind _asbp_weapon_sword (Utilities|Casting|CastToBP_Weapon_Sword (Variables|/Script/Engine.ChildActorComponent|GetChildActor (Variables|Default|GetSword_Right))))
  (Transformation|DetachFromActor _asbp_weapon_sword "KeepWorld" "KeepWorld" "KeepWorld")
  (Physics|SetSimulatePhysics (Variables|/Game/Blueprints/Items/BP_Weapon_Sword.BP_Weapon_Sword_C|GetSword _asbp_weapon_sword) true))

(fn ConstructionScript
  (bind _sword_right (Variables|Default|GetSword_Right))
  (bind _childactor (Variables|/Script/Engine.ChildActorComponent|GetChildActor _sword_right))
  (|CallParentFunction)
  (Variables|Default|SetRightHandItem _childactor)
  (Actor|SetOwner _childactor self))