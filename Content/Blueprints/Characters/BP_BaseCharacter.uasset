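; BP_BaseCharacter is a base character Blueprint that provides melee attack routing, health and death.
; Melee start and end events pick the right hand, left hand or mouth item by attack type and message it through BPI_Item.
; Damage not instigated by its own controller lowers Health, triggering Death once at zero or below.
; Death ragdolls the mesh, disables capsule collision, then disables player input or destroys the AI controller.
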(event Custom|Death
  (bind _returnvalue (Pawn|GetController))
  (bind _mesh (Variables|Character|GetMesh))
  ;[1 1 1] Death
  (Variables|Default|SetDead true)
  (Class|SkeletalMeshComponent|SetAllBodiesSimulatePhysics _mesh true)
  (Collision|SetCollisionEnabled _mesh "QueryAndPhysics")
  (Collision|SetCollisionEnabled (Variables|Collision|GetCapsuleComponent) "NoCollision")
  (bind _asplayer_controller (Utilities|Casting|CastToPlayerController _returnvalue)
    (:then
      (Input|DisableInput _asplayer_controller))
    (:CastFailed
      (bind _asaicontroller (Utilities|Casting|CastToAIController _returnvalue))
      (Actor|DestroyActor _asaicontroller))))

(event Custom|MeleeAttackStart
  (params (MeleeAttackType :type EnumMeleeAttackType%20Enum :default "NewEnumerator2"))
  (bind _righthanditem (Variables|Default|GetRightHandItem))
  (bind _lefthanditem (Variables|Default|GetLeftHandItem))
  (bind _mouthitem (Variables|Default|GetMouthItem))
  (bind _returnvalue (Utilities|Select :Index MeleeAttackType :NewEnumerator2 _righthanditem :NewEnumerator1 _lefthanditem :NewEnumerator0 _mouthitem))
  ;[1 1 1] Start/End Attack
  (Utilities|IsValid _returnvalue
    (:Is%20Valid
      (if (Utilities|DoesObjectImplementInterface _returnvalue "/Game/Blueprints/Items/BPI_Item.BPI_Item_C")
        (Class|BPIItem|StartAttack(Message) _returnvalue)))))

(event Custom|MeleeAttackEnd
  (params (MeleeAttackType :type EnumMeleeAttackType%20Enum :default "NewEnumerator2"))
  (bind _righthanditem (Variables|Default|GetRightHandItem))
  (bind _lefthanditem (Variables|Default|GetLeftHandItem))
  (bind _mouthitem (Variables|Default|GetMouthItem))
  (bind _returnvalue (Utilities|Select :Index MeleeAttackType :NewEnumerator2 _righthanditem :NewEnumerator1 _lefthanditem :NewEnumerator0 _mouthitem))
  ;[1 1 1] Start/End Attack
  (Utilities|IsValid _returnvalue
    (:Is%20Valid
      (if (Utilities|DoesObjectImplementInterface _returnvalue "/Game/Blueprints/Items/BPI_Item.BPI_Item_C")
        (Class|BPIItem|EndAttack(Message) _returnvalue)))))

(event Game|Damage|EventAnyDamage
  (params (Damage :type Float%20%28single-precision%29) (DamageType :type Damage%20Type%20Object%20Reference) (InstigatedBy :type Controller%20Object%20Reference) (DamageCauser :type Actor%20Object%20Reference))
  ;[1 1 1] Damage
  (if (!= InstigatedBy (Pawn|GetController))
    (bind _output_get (Variables|Default|SetHealth (- (Variables|Default|GetHealth) Damage)))
    (if (and (<= _output_get 0.0) (not (Variables|Default|GetDead)))
      (CallFunction|Death))))

(fn ConstructionScript)