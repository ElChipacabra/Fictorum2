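; BP_NPC is an NPC character Blueprint that handles attack animations, with server and multicast events implied by their names.
; Server_NPC_Attack picks a random entry from AttackMontages and passes it to MC_NPC_Attack.
; The multicast event ignores that argument, playing a hard-coded montage on the Mesh and printing the PlayMontage result.
; A PlayAnimMontage node using the argument is left unwired, and BeginPlay, overlap and Tick are disabled.
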(event Custom|MC_NPC_Attack
  (params (AnimMontage :type Anim%20Montage%20Object%20Reference))
  (bind _notifyname (Animation|Montage|PlayMontage (Variables|Character|GetMesh) "/Game/Characters/Mannequins/Animations/Manny/SwordAnimPro/2xAttack_Move_med_Rdown_L_1_Retargeted_Montage.2xAttack_Move_med_Rdown_L_1_Retargeted_Montage")
    (:then
      (Development|PrintString (Utilities|String|ToString(Name) _notifyname)))))

(event Custom|Server_NPC_Attack
  (CallFunction|MCNPCAttack (.OutItem (Utilities|Array|Random (Variables|Default|GetAttackMontages)))))

(event EventBeginPlay
  (|CallParentFunction) ; This node is disabled and will not be called.\nDrag off pins to build functionality.
)

(event Collision|EventActorBeginOverlap
  (params (OtherActor :type Actor%20Object%20Reference))
  (|CallParentFunction OtherActor) ; This node is disabled and will not be called.\nDrag off pins to build functionality.
)

(event EventTick
  (params (DeltaSeconds :type Float%20%28single-precision%29))
  (|CallParentFunction DeltaSeconds) ; This node is disabled and will not be called.\nDrag off pins to build functionality.
)

(fn ConstructionScript
  (|CallParentFunction))