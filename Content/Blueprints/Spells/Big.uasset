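; Big is a spell Blueprint that produces an explosion on Chaos destructibles through physics fields.
; Explode_Event first applies a very strong, uniform external cluster strain field sized and centered on its Sphere component to fracture geometry.
; It then applies a radial linear force from the same center to scatter the pieces.
; Nothing in the graph calls the event, so it relies on an outside trigger.
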(event Custom|Explode_Event
  (bind _sphere (Variables|Default|GetSphere))
  (bind _returnvalue (Transformation|GetWorldLocation _sphere))
  (Class|FieldSystemComponent|ApplyPhysicsField (Variables|Field|GetFieldSystemComponent) true "Field_ExternalClusterStrain" 0 (Field|SetRadialFalloff (Variables|Default|GetRadialFalloff) 5e+07 0.0 1.0 0.0 (Components|Sphere|GetScaledSphereRadius _sphere) _returnvalue "Field_FallOff_None"))
  (Class|FieldSystemComponent|ApplyPhysicsField (Variables|Field|GetFieldSystemComponent) true "Field_LinearForce" 0 (Field|SetRadialVector (Variables|Default|GetRadialVector) 2.5e+09 _returnvalue)))

(event Collision|EventActorBeginOverlap
  (params (OtherActor :type Actor%20Object%20Reference)))

(event EventTick
  (params (DeltaSeconds :type Float%20%28single-precision%29)))

(fn ConstructionScript)