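; Melee weapon item that damages an actor overlapped by its capsule hitbox during an attack.
; StartAttack enables and shows the capsule, EndAttack disables and hides it, and BeginPlay starts it in the ended state.
; Overlaps ignore the owner and pass a DoOnce, reset on each start and end, so each swing applies fixed damage once, credited to the owning Character's controller.
; The construction script sizes the capsule from variables.
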(event Custom|MeleeOverlap
  (params (OverlappedComponent :type Primitive%20Component%20Object%20Reference) (OtherActor :type Actor%20Object%20Reference) (OtherComp :type Primitive%20Component%20Object%20Reference) (OtherBodyIndex :type Integer) (bFromSweep :type Boolean) (SweepResult :type Hit%20Result%20Structure%20%28by%20ref%29))
  (if (!= OtherActor (Components|GetOwner))
    (Utilities|FlowControl|DoOnce false
      (:Completed
        (bind _ascharacter (Utilities|Casting|CastToCharacter (Components|GetOwner)))
        (Game|Damage|ApplyDamage OtherActor 1e+01 (Pawn|GetController _ascharacter) self)))))

(event EventBeginPlay
  (|CallParentFunction)
  (Collision|BindEventtoOnComponentBeginOverlap (Variables|Default|GetCapsule) (EventDispatchers|CreateEvent :!event Custom|MeleeOverlap))
  (CallFunction|EndAttack))

(event EventStartAttack
  (bind _capsule (Variables|Default|GetCapsule))
  (bind _capsule_2 (Variables|Default|GetCapsule))
  (Collision|SetCollisionEnabled _capsule "QueryOnly")
  (Development|SetHiddeninGame _capsule false false)
  (Rendering|SetVisibility _capsule true false)
  (Utilities|FlowControl|Sequence
    (:then_0
      (Utilities|FlowControl|DoOnce false
        (:Completed
          (Variables|/Script/Engine.PrimitiveComponent|SetbGenerateOverlapEvents _capsule_2 true)
          (Collision|SetCollisionObjectType _capsule_2 "ECC_Pawn")
          (Collision|SetCollisionResponsetoChannel _capsule_2 "ECC_Pawn" "ECR_Overlap")
          (Collision|SetCollisionObjectType _capsule_2 "ECC_Pawn"))))
    (:then_1
      (Utilities|FlowControl|DoOnce false) ; enters at Reset
    )))

(event EventEndAttack
  (bind _capsule (Variables|Default|GetCapsule))
  (bind _capsule_2 (Variables|Default|GetCapsule))
  (Collision|SetCollisionEnabled _capsule "NoCollision")
  (Development|SetHiddeninGame _capsule true false)
  (Rendering|SetVisibility _capsule false false)
  (Utilities|FlowControl|Sequence
    (:then_0
      (Utilities|FlowControl|DoOnce false
        (:Completed
          (Variables|/Script/Engine.PrimitiveComponent|SetbGenerateOverlapEvents _capsule_2 true)
          (Collision|SetCollisionObjectType _capsule_2 "ECC_Pawn")
          (Collision|SetCollisionResponsetoChannel _capsule_2 "ECC_Pawn" "ECR_Overlap")
          (Collision|SetCollisionObjectType _capsule_2 "ECC_Pawn"))))
    (:then_1
      (Utilities|FlowControl|DoOnce false) ; enters at Reset
    )))

(fn ConstructionScript
  (Components|Capsule|SetCapsuleRadius (Variables|Default|GetCapsule) (Variables|Default|GetCapsuleRadius) true)
  (Components|Capsule|SetCapsuleHalfHeight (Variables|Default|GetCapsule) (Variables|Default|GetCapsuleHalfHeight) true))