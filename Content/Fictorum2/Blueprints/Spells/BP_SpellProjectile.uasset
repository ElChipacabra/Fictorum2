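; Spell projectile actor that deals direct and radial damage when its collision sphere hits something.
; On hit it stops its trail effects, spawns an explosion emitter, disables collision and expires after a short delay.
; The construction script fills an ignore list with all Player-tagged base characters when the instigator is a player, sparing them from both damage types.
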(event OnComponentHit(Sphere)
  (params (HitComponent :type Primitive%20Component%20Object%20Reference) (OtherActor :type Actor%20Object%20Reference) (OtherComp :type Primitive%20Component%20Object%20Reference) (NormalImpulse :type Vector :default "0, 0, 0") (Hit :type Hit%20Result%20Structure%20%28by%20ref%29))
  (bind _location (Collision|BreakHitResult Hit))
  (Components|Activation|Deactivate (Variables|Default|GetNiagara))
  (if (not (Utilities|Array|ContainsItem (Variables|Default|GetIgnoreActors) OtherActor))
    (Game|Damage|ApplyDamage OtherActor 1e+01 0 0))
  (Game|Damage|ApplyRadialDamage 2e+01 _location 1e+02 "/Script/Engine.DamageType" (Variables|Default|GetIgnoreActors) self (Pawn|GetController (Variables|Actor|GetInstigator)) false "ECC_Visibility")
  (Effects|SpawnEmitteratLocation "/Game/StarterContent/Particles/P_Explosion.P_Explosion" _location)
  (Collision|SetActorEnableCollision false)
  (Actor|SetLifeSpan 1.0))

(event EventBeginPlay)

(event Collision|EventActorBeginOverlap
  (params (OtherActor :type Actor%20Object%20Reference)))

(event EventTick
  (params (DeltaSeconds :type Float%20%28single-precision%29)))

(fn ConstructionScript
  (CallFunction|SetIgnoreActors))

(fn SetIgnoreActors
  (bind _instigator (Variables|Actor|GetInstigator))
  (Utilities|IsValid _instigator
    (:Is%20Valid
      (if (Actor|ActorHasTag _instigator "Player")
        (bind _outactors (Actor|GetAllActorsOfClasswithTag "/Game/Fictorum2/Blueprints/Characters/BP_FictorumBaseCharacter.BP_FictorumBaseCharacter_C" "Player"))
        (Variables|Default|SetIgnoreActors _outactors)))))