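; BP_FictorumGameMode is the game mode that sets up two playable characters, a Wizard and a Spirit Wolf.
; On BeginPlay it spawns the Wizard and Wolf at the first and second PlayerStart found and stores both references.
; Each new player, after a short delay, possesses the Wizard, or the Wolf if the Wizard is already player-controlled.
; GetOtherPlayer returns the partner character; a disconnected Wolf spawn remains unused.
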(event EventHandleStartingNewPlayer
  (params (NewPlayer :type Player%20Controller%20Object%20Reference))
  (bind _wizard (Variables|Default|GetWizard))
  ;[1 1 1] Possessing Wizard if it's available, if not possessing Wolf
  (Utilities|FlowControl|Delay 0.2)
  (if (Pawn|IsPlayerControlled _wizard)
    (Pawn|Possess NewPlayer (Variables|Default|GetWolf))
    (else
      (Pawn|Possess NewPlayer _wizard))))

(event EventBeginPlay
  ;[0 1 0] Spawning both actors on Begin Play
  (bind _outactors (Actor|GetAllActorsOfClass "/Script/Engine.PlayerStart"))
  (for (_array_element _array_index) _outactors
    (switch int _array_index
      (:0
        (bind _returnvalue (Game|SpawnActorfromClass "/Game/Fictorum2/Blueprints/Characters/BP_FictorumPlayerCharacter.BP_FictorumPlayerCharacter_C" (Math|Transform|MakeTransform (.location (Transformation|GetActorTransform _array_element)) (.rotation (Transformation|GetActorTransform _array_element)) "1.000000,1.000000,1.000000") "Undefined" "MultiplyWithRoot" 0 0))
        (Variables|Default|SetWizard _returnvalue))
      (:1
        (bind _returnvalue_2 (Game|SpawnActorfromClass "/Game/Fictorum2/Blueprints/Characters/BP_SpiritWolf.BP_SpiritWolf_C" (Math|Transform|MakeTransform (.location (Transformation|GetActorTransform _array_element)) (.rotation (Transformation|GetActorTransform _array_element)) "1.000000,1.000000,1.000000") "Undefined" "MultiplyWithRoot" 0 0))
        (Variables|Default|SetWolf _returnvalue_2)))))

(fn ConstructionScript)

(fn GetOtherPlayer
  (params (Player :type Actor%20Object%20Reference))
  (bind _wizard (Variables|Default|GetWizard))
  (return (select (== _wizard Player) (Variables|Default|GetWolf) _wizard)))