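; BP_SpiritWolf is a spirit wolf character whose melee attack is a bite.
; A bite hit event applies fixed damage to the hit actor through a DoOnce gate, which resets when the melee attack ends, so each attack damages once.
; The construction script stores the Bite child actor as the mouth item and sets the wolf as its owner.
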(event Custom|MeleeHit_Bite
  (params (OverlappedComponent :type Primitive%20Component%20Object%20Reference) (OtherActor :type Actor%20Object%20Reference) (OtherComp :type Primitive%20Component%20Object%20Reference) (OtherBodyIndex :type Integer) (bFromSweep :type Boolean) (SweepResult :type Hit%20Result%20Structure%20%28by%20ref%29))
  (Utilities|FlowControl|DoOnce false
    (:Completed
      (Game|Damage|ApplyDamage OtherActor 1e+01 (Pawn|GetController) self))))

(event EventMeleeAttackEnd
  (params (MeleeAttackType :type EnumMeleeAttackType%20Enum :default "NewEnumerator2"))
  (|CallParentFunction MeleeAttackType)
  (Utilities|FlowControl|DoOnce false) ; enters at Reset
)

(fn ConstructionScript
  (bind _bite (Variables|Default|GetBite))
  (bind _childactor (Variables|/Script/Engine.ChildActorComponent|GetChildActor _bite))
  (|CallParentFunction)
  (Variables|Default|SetMouthItem _childactor)
  (Actor|SetOwner _childactor self))