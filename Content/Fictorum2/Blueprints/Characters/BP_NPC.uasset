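; BP_NPC is a Blueprint for NPC characters that handles melee attack animation and death cleanup.
; A server attack event picks a random melee montage and passes it to a multicast event that plays it on the mesh.
; On server death, it runs the parent logic, clears the mesh's animation class and, if despawning is enabled, sets a random lifespan within the configured time range.
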(event Custom|MC_NPC_Attack
  (params (AnimMontage :type Anim%20Montage%20Object%20Reference))
  (Animation|Montage|PlayMontage (Variables|Character|GetMesh) AnimMontage))

(event Custom|Server_NPC_Attack
  (CallFunction|MCNPCAttack (.OutItem (Utilities|Array|Random (Variables|Default|GetMeleeAttackMontages)))))

(event EventBeginPlay
  (|CallParentFunction) ; This node is disabled and will not be called.\nDrag off pins to build functionality.
)

(event EventDeathServer
  (bind _despawntimerange (Variables|Default|GetDespawnTimeRange))
  (bind (_x _y) (Math|Vector2D|BreakVector2D _despawntimerange))
  (|CallParentFunction)
  (Class|SkeletalMeshComponent|SetAnimClass (Variables|Character|GetMesh))
  (if (Variables|Default|GetDespawn)
    (Actor|SetLifeSpan (Math|Random|RandomFloatinRange _x _y))))

(fn ConstructionScript
  (|CallParentFunction))