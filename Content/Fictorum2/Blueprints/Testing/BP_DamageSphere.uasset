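; BP_DamageSphere is a testing actor that deals periodic damage to Characters inside a spherical volume.
; On BeginPlay it starts a looping one-second timer that applies DamagePerSec to every overlapping Character.
; The construction script scales the Sphere component from the collision sphere's radius, presumably so the visual matches the damage area.
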(event Custom|DamageAllActors
  (for _array_element (Collision|GetOverlappingActors "/Script/Engine.Character" :!class /Script/Engine.Actor)
    (Game|Damage|ApplyDamage _array_element (Variables|Default|GetDamagePerSec) 0 0)))

(event EventBeginPlay
  (Utilities|Time|SetTimerbyEvent (delegate Custom|DamageAllActors) 1.0 true))

(event Collision|EventActorBeginOverlap
  (params (OtherActor :type Actor%20Object%20Reference)))

(event EventTick
  (params (DeltaSeconds :type Float%20%28single-precision%29)))

(fn ConstructionScript
  (bind _assphere_collision (Utilities|Casting|CastToSphereComponent (Variables|Default|GetCollisionComponent)))
  (Transformation|SetWorldScale3D (Variables|Default|GetSphere) (Math|Conversions|ToVector(Float) (/ (Variables|/Script/Engine.SphereComponent|GetSphereRadius _assphere_collision) 5e+01))))